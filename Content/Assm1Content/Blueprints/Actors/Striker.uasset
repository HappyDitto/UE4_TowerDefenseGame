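; Striker is a ranged attacker that turns to face its first attack target and fires bullets at it.
; It extends a parent class, setting its attack stats in the construction script and adding yaw-only tracking on Tick.
; Attack calls GenerateBullet, which spawns an St_Bullet through SpawnAIFromClass and passes it the damage range, flight speed, hit radius and target, then plays a 2D firing sound.
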(event EventTick
  (params (DeltaSeconds :type Float%20%28single-precision%29))
  (|CallParentFunction 0.0)
  (if (> (Utilities|Array|Length (Variables|Default|GetattackTargets)) 0)
    (Transformation|SetActorRotation (Math|Rotator|MakeRotator 0.0 0.0 (.yaw (Math|Rotator|FindLookatRotation (Transformation|GetActorLocation) (Transformation|GetActorLocation (Utilities|Array|Get(acopy) (Variables|Default|GetattackTargets)))))))))

(event EventAttack
  (params (Target :type Enemy%20Object%20Reference))
  (CallFunction|GenerateBullet)
  (Audio|PlaySound2D "/Game/Assm1Content/Resources/sounds/striker.striker" 0.25 0.7 0.0 0 0))

(fn ConstructionScript
  (Variables|Default|SetmaxAttackDamage 35.0)
  (Variables|Default|SetattackSpeed 1.25)
  (Variables|Default|SetattackRadius 4.0)
  (Variables|Default|SetminAttackDamage 25.0)
  (|CallParentFunction))

(fn GenerateBullet
  (bind _returnvalue (AI|SpawnAIFromClass "/Game/Assm1Content/Blueprints/Actors/St_Bullet.St_Bullet_C" 0 (Transformation|GetActorLocation) "0, 0, 0" false))
  (bind _asst_bullet (Utilities|Casting|CastToSt_Bullet _returnvalue))
  (Variables|/Game/Assm1Content/Blueprints/Actors/St_Bullet.St_Bullet_C|SetmaxAttackDamage _asst_bullet (Variables|Default|GetmaxAttackDamage))
  (Variables|/Game/Assm1Content/Blueprints/Actors/St_Bullet.St_Bullet_C|SetminAttackDamage _asst_bullet (Variables|Default|GetminAttackDamage))
  (Variables|/Game/Assm1Content/Blueprints/Actors/St_Bullet.St_Bullet_C|SetflySpeed _asst_bullet 5e+02)
  (Variables|/Game/Assm1Content/Blueprints/Actors/St_Bullet.St_Bullet_C|SetattackRadius _asst_bullet 75.0)
  (Variables|/Game/Assm1Content/Blueprints/Actors/St_Bullet.St_Bullet_C|Settarget _asst_bullet (Utilities|Array|Get(acopy) (Variables|Default|GetattackTargets))))