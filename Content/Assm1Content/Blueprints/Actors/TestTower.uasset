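; TestTower is a tower actor that automatically damages Enemy actors within its range.
; Overlap events add and remove enemies from a target array, and the construction script scales the AttackRange component from AttackRadius, stretched vertically.
; A looping timer at the AttackSpeed interval attacks the first target in the array, subtracting random damage from its health, calling BeAttacked and playing a sound.
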(event Custom|AttackEnemy
  (CallFunction|SetUpAttack))

(event EventBeginPlay
  (Utilities|Time|SetTimerbyEvent (delegate Custom|AttackEnemy) (Variables|Default|GetattackSpeed) true))

(event Collision|EventActorBeginOverlap
  (params (OtherActor :type Actor%20Object%20Reference))
  (if (== (Utilities|GetClass OtherActor) "/Game/Assm1Content/Blueprints/Actors/Enemy.Enemy_C")
    (bind _asenemy (Utilities|Casting|CastToEnemy OtherActor))
    (Utilities|Array|Add (Variables|Default|GetattackTargets) _asenemy)))

(event Collision|EventActorEndOverlap
  (params (OtherActor :type Actor%20Object%20Reference))
  (if (== (Utilities|GetClass OtherActor) "/Game/Assm1Content/Blueprints/Actors/Enemy.Enemy_C")
    (bind _asenemy (Utilities|Casting|CastToEnemy OtherActor))
    (Utilities|Array|RemoveItem (Variables|Default|GetattackTargets) _asenemy)))

(fn ConstructionScript
  (bind _attackradius (Variables|Default|GetattackRadius))
  (Transformation|SetWorldScale3D (Variables|Default|GetAttackRange) (Math|Vector|MakeVector _attackradius _attackradius (* _attackradius 3.0))))

(fn Attack
  (params (Target :type Enemy%20Object%20Reference))
  (Utilities|IsValid Target
    (:Is%20Valid
      (Variables|/Game/Assm1Content/Blueprints/Actors/Enemy.Enemy_C|SetCurrentHealth Target (- (Variables|/Game/Assm1Content/Blueprints/Actors/Enemy.Enemy_C|GetCurrentHealth Target) (Math|Random|RandomFloatinRange (Variables|Default|GetminAttackDamage) (Variables|Default|GetmaxAttackDamage))))
      (Default|BeAttacked Target)
      (Audio|PlaySound2D "/Game/Assm1Content/Resources/sounds/sentinel.sentinel" 1.0 1.0 0.0 0 0))
    (:Is%20Not%20Valid
      (return))))

(fn SetUpAttack
  (if (not (== (Utilities|Array|Length (Variables|Default|GetattackTargets)) 0))
    (CallFunction|Attack (Utilities|Array|Get(acopy) (Variables|Default|GetattackTargets)))))