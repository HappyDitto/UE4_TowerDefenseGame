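; SpawnAI is a spawner actor that creates a random enemy at its own location every two seconds on a looping timer.
; The construction script fills lookup maps for health, speed, gold and material across four tiers, where tougher tiers move slower and pay more gold.
; GenerateEnemy picks a random tier, spawns an Enemy and applies those values, then the spawn event calls Constructed and assigns one of four routes at random.
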(event Custom|Spawn%20Enemy
  (bind _generatedenemy (CallFunction|GenerateEnemy))
  (Default|Constructed _generatedenemy)
  (switch int (Math|Random|RandomInteger 4)
    (:Default
      (Variables|/Game/Assm1Content/Blueprints/Actors/Enemy.Enemy_C|SetRoute _generatedenemy (Variables|Default|GetRoute1) :!label _label))
    (:0
      (goto _label))
    (:1
      (Variables|/Game/Assm1Content/Blueprints/Actors/Enemy.Enemy_C|SetRoute _generatedenemy (Variables|Default|GetRoute2)))
    (:2
      (Variables|/Game/Assm1Content/Blueprints/Actors/Enemy.Enemy_C|SetRoute _generatedenemy (Variables|Default|GetRoute3)))
    (:3
      (Variables|/Game/Assm1Content/Blueprints/Actors/Enemy.Enemy_C|SetRoute _generatedenemy (Variables|Default|GetRoute4)))))

(event EventBeginPlay
  (Utilities|Time|SetTimerbyEvent (delegate Custom|Spawn%20Enemy) 2.0 true))

(fn ConstructionScript
  (Utilities|Map|Add (Variables|Default|GetHEALTH_DIC) 1 25.0)
  (Utilities|Map|Add (Variables|Default|GetHEALTH_DIC) 2 5e+01)
  (Utilities|Map|Add (Variables|Default|GetHEALTH_DIC) 3 75.0)
  (Utilities|Map|Add (Variables|Default|GetHEALTH_DIC) 4 1e+02)
  (Utilities|Map|Add (Variables|Default|GetSPEED_DIC) 1 1.2e+02)
  (Utilities|Map|Add (Variables|Default|GetSPEED_DIC) 2 9e+01)
  (Utilities|Map|Add (Variables|Default|GetSPEED_DIC) 3 6e+01)
  (Utilities|Map|Add (Variables|Default|GetSPEED_DIC) 4 3e+01)
  (Utilities|Map|Add (Variables|Default|GetGOLD_DIC) 1 5)
  (Utilities|Map|Add (Variables|Default|GetGOLD_DIC) 2 10)
  (Utilities|Map|Add (Variables|Default|GetGOLD_DIC) 3 15)
  (Utilities|Map|Add (Variables|Default|GetGOLD_DIC) 4 20)
  (Utilities|Map|Add (Variables|Default|GetMATERIAL_DIC) 1 "/Game/Assm1Content/Materials/M_UE4Man_Blue.M_UE4Man_Blue")
  (Utilities|Map|Add (Variables|Default|GetMATERIAL_DIC) 2 "/Game/Assm1Content/Materials/M_UE4Man_Green.M_UE4Man_Green")
  (Utilities|Map|Add (Variables|Default|GetMATERIAL_DIC) 3 "/Game/Mannequin/Character/Materials/M_UE4Man_Body.M_UE4Man_Body")
  (Utilities|Map|Add (Variables|Default|GetMATERIAL_DIC) 4 "/Game/Assm1Content/Materials/M_UE4Man_Red.M_UE4Man_Red"))

(fn GenerateEnemy
  (Variables|Default|SetcurrentEnemyType (+ (Math|Random|RandomInteger 4) 1))
  (bind _returnvalue (AI|SpawnAIFromClass "/Game/Assm1Content/Blueprints/Actors/Enemy.Enemy_C" 0 (Transformation|GetActorLocation) "0, 0, 0" false))
  (bind _asenemy (Utilities|Casting|CastToEnemy _returnvalue))
  (Variables|/Game/Assm1Content/Blueprints/Actors/Enemy.Enemy_C|SetMaxHealth _asenemy (.Value (Utilities|Map|Find (Variables|Default|GetHEALTH_DIC) (Variables|Default|GetcurrentEnemyType))))
  (Variables|/Game/Assm1Content/Blueprints/Actors/Enemy.Enemy_C|SetSpeed _asenemy (.Value (Utilities|Map|Find (Variables|Default|GetSPEED_DIC) (Variables|Default|GetcurrentEnemyType))))
  (Variables|/Game/Assm1Content/Blueprints/Actors/Enemy.Enemy_C|SetGold _asenemy (.Value (Utilities|Map|Find (Variables|Default|GetGOLD_DIC) (Variables|Default|GetcurrentEnemyType))))
  (Rendering|Material|SetMaterial (Variables|/Script/Engine.Character|GetMesh _asenemy) 0 (.Value (Utilities|Map|Find (Variables|Default|GetMATERIAL_DIC) (Variables|Default|GetcurrentEnemyType))))
  (return _asenemy))