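; Sentinel is an attacking actor, derived from a parent class, that hits every target in its AttackTargets list.
; Its construction script sets damage range, attack speed and radius before calling the parent's.
; SetUpAttack activates the Bullet component and calls Attack on each target.
; Tick and end-overlap, which runs the parent's handling first, deactivate Bullet once no targets remain.
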(event EventSetUpAttack
  (Components|Activation|SetActive (Variables|Default|Getbullet) true false)
  (for _array_element (Variables|Default|GetattackTargets)
    (CallFunction|Attack _array_element)))

(event Collision|EventActorEndOverlap
  (params (OtherActor :type Actor%20Object%20Reference))
  (|CallParentFunction OtherActor)
  (if (== (Utilities|Array|Length (Variables|Default|GetattackTargets)) 0)
    (Components|Activation|SetActive (Variables|Default|Getbullet) false false)))

(event EventTick
  (params (DeltaSeconds :type Float%20%28single-precision%29))
  (if (== (Utilities|Array|Length (Variables|Default|GetattackTargets)) 0)
    (Components|Activation|SetActive (Variables|Default|Getbullet) false false)))

(fn ConstructionScript
  (Variables|Default|SetmaxAttackDamage 25.0)
  (Variables|Default|SetattackSpeed 0.75)
  (Variables|Default|SetattackRadius 5.0)
  (Variables|Default|SetminAttackDamage 15.0)
  (|CallParentFunction))