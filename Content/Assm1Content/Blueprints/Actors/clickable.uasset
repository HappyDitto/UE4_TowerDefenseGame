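; Clickable build-slot actor that lets the player choose a Sentinel or Striker tower to construct on it.
; BeginPlay links two TowerButton widget components to this actor and their tower types, and enables player input.
; Clicking the panel shows both buttons when CanConstruct is true, otherwise shows a disabled material.
; Left mouse presses or button releases hide the buttons, while cursor and click events swap panel materials for feedback.
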(event OnClicked(Plane)
  (params (TouchedComponent :type Primitive%20Component%20Object%20Reference) (ButtonPressed :type Key%20Structure))
  (bind _plane (Variables|Default|GetPlane))
  (if (Variables|Default|GetcanConstruct)
    (Rendering|Material|SetMaterial _plane 0 "/Game/Assm1Content/Materials/M_Tech_Panel_Clicked.M_Tech_Panel_Clicked")
    (Rendering|SetVisibility (Variables|Default|GetSentinelGenerator) true false)
    (Rendering|SetVisibility (Variables|Default|GetStrikerGenerator) true false)
    (else
      (Rendering|Material|SetMaterial _plane 0 "/Game/Assm1Content/Materials/M_Tech_Panel_Disabled.M_Tech_Panel_Disabled"))))

(event Custom|ButtonReleased
  (params (TouchedActor :type Actor%20Object%20Reference) (ButtonReleased :type Key%20Structure))
  (Rendering|SetVisibility (Variables|Default|GetSentinelGenerator) false false)
  (Rendering|SetVisibility (Variables|Default|GetStrikerGenerator) false false))

(event EventBeginPlay
  (CallFunction|InitButton (Variables|Default|GetSentinelGenerator) "/Game/Assm1Content/Blueprints/Actors/Sentinel.Sentinel_C")
  (CallFunction|InitButton (Variables|Default|GetStrikerGenerator) "/Game/Assm1Content/Blueprints/Actors/Striker.Striker_C")
  (Input|EnableInput (Game|GetPlayerController 0)))

(event MouseInput|EventActorBeginCursorOver
  (Rendering|Material|SetMaterial (Variables|Default|GetPlane) 0 "/Game/Assm1Content/Materials/M_Tech_Panel_Over.M_Tech_Panel_Over"))

(event EventActorOnReleased
  (params (ButtonReleased :type Key%20Structure))
  (Utilities|FlowControl|Delay 0.2)
  (Rendering|Material|SetMaterial (Variables|Default|GetPlane) 0 "/Game/Assm1Content/Materials/M_Tech_Panel_Over.M_Tech_Panel_Over"))

(event MouseInput|EventActorEndCursorOver
  (Rendering|Material|SetMaterial (Variables|Default|GetPlane) 0 "/Game/Assm1Content/Materials/M_Tech_Panel.M_Tech_Panel"))

(event Input|MouseEvents|LeftMouseButton
  (params (Key :type Key%20Structure))
  (:Pressed
    (Development|PrintString "Hello")
    (Rendering|SetVisibility (Variables|Default|GetSentinelGenerator) false true)
    (Rendering|SetVisibility (Variables|Default|GetStrikerGenerator) false true)))

(fn ConstructionScript)

(fn InitButton
  (params (widget :type Widget%20Component%20Object%20Reference) (towerGenerated :type Actor%20Class%20Reference))
  (bind _astower_button (Utilities|Casting|CastToTowerButton (UserInterface|GetUserWidgetObject widget)))
  (Variables|/Game/Assm1Content/UI/TowerButton.TowerButton_C|SetClickable _astower_button self)
  (Variables|/Game/Assm1Content/UI/TowerButton.TowerButton_C|SetTowerOfButtonFor _astower_button towerGenerated))