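; BP_TD_GameState is a game state Blueprint that tracks Life, Score and Gold for the TD game mode.
; LoseLife decrements Life and, when it equals exactly zero, casts to BP_TD_GameMode and calls GameOver.
; AddScore increments Score by one.
; AddGold and LoseGold both add the passed Value to Gold, so LoseGold reduces it only when given a negative amount.
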(event Custom|AddScore
  (Variables|Default|Setscore (+ (Variables|Default|Getscore) 1)))

(event Custom|LoseLife
  (bind _output_get (Variables|Default|Setlife (- (Variables|Default|Getlife) 1)))
  (if (== _output_get 0)
    (bind _asbp_td_game_mode (Utilities|Casting|CastToBP_TD_GameMode (Game|GetGameMode)))
    (Default|GameOver _asbp_td_game_mode)))

(fn ConstructionScript)

(fn AddGold
  (params (Value :type Integer%20%28by%20ref%29))
  (Variables|Default|Setgold (+ Value (Variables|Default|Getgold))))

(fn LoseGold
  (params (Value :type Integer%20%28by%20ref%29))
  (Variables|Default|Setgold (+ Value (Variables|Default|Getgold))))