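; Game mode for a tower defense game that sets up the session, handles pausing and ends the game.
; On BeginPlay it creates the pause and game UI widgets, enables mouse cursor input and seeds Life, Score and Gold on BP_TD_GameState from its initial values.
; The P key toggles pause with the pause widget and a camera fade.
; GameOver pauses, clears widgets, disables input and shows the game-over screen with the same fade.
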(event Custom|GameOver
  (bind _returnvalue (Game|GetPlayerController 0))
  (Game|SetGamePaused true)
  (Viewport|RemoveAllWidgets)
  (Input|DisableInput _returnvalue)
  (bind _returnvalue_2 (UserInterface|CreateWidget "/Game/Assm1Content/UI/GameOver.GameOver_C" _returnvalue))
  (UserInterface|Viewport|AddtoViewport _returnvalue_2 0)
  (Class|PlayerCameraManager|SetManualCameraFade (Game|GetPlayerCameraManager 0) 0.7 "(R=0.000000,G=0.000000,B=0.000000,A=0.500000)" false))

(event EventBeginPlay
  (bind _returnvalue (Game|GetPlayerController 0))
  (bind _returnvalue_2 (UserInterface|CreateWidget "/Game/Assm1Content/UI/Pause.Pause_C" _returnvalue))
  (UserInterface|Viewport|AddtoViewport _returnvalue_2 0)
  (Input|EnableInput _returnvalue)
  (Variables|/Script/Engine.PlayerController|SetbShowMouseCursor _returnvalue true)
  (Variables|/Script/Engine.PlayerController|SetbEnableMouseOverEvents _returnvalue true)
  (Variables|/Script/Engine.PlayerController|SetbEnableClickEvents _returnvalue true)
  (bind _asbp_td_game_state (Utilities|Casting|CastToBP_TD_GameState (Game|GetGameState)))
  (Variables|/Game/Assm1Content/Blueprints/BP_TD_GameState.BP_TD_GameState_C|Setlife _asbp_td_game_state (Variables|Default|GetInitLife))
  (Variables|/Game/Assm1Content/Blueprints/BP_TD_GameState.BP_TD_GameState_C|Setscore _asbp_td_game_state (Variables|Default|GetInitScore))
  (Variables|/Game/Assm1Content/Blueprints/BP_TD_GameState.BP_TD_GameState_C|Setgold _asbp_td_game_state (Variables|Default|GetInitMoney))
  (bind _returnvalue_3 (UserInterface|CreateWidget "/Game/Assm1Content/UI/GameUI.GameUI_C" (Game|GetPlayerController 0)))
  (UserInterface|Viewport|AddtoViewport _returnvalue_3 0))

(event Input|KeyboardEvents|P
  (params (Key :type Key%20Structure))
  (bind _returnvalue (Game|GetPlayerCameraManager 0))
  (:Pressed
    (Game|SetGamePaused (not (Game|IsGamePaused)))
    (if (Game|IsGamePaused)
      (Widget|SetVisibility (stale EventBeginPlay _returnvalue_2) "Visible")
      (Class|PlayerCameraManager|SetManualCameraFade _returnvalue 0.7 "(R=0.000000,G=0.000000,B=0.000000,A=0.500000)" false)
      (else
        (Widget|SetVisibility (stale EventBeginPlay _returnvalue_2) "Hidden")
        (CameraFades|StopCameraFade _returnvalue)))))

(fn ConstructionScript)